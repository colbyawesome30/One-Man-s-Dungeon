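; Quest-giver NPC that the player talks to through the interaction system to accept and complete one of three quests, selected by QuestID.
; StartDialogue positions and locks the player, switches view to the NPC and opens WBP_DIalogue at StartRow.
; DialogueHandler updates StartRow and PlayerGameInstance objectives; IsQuestDone also spawns rewards as it checks completion.
; Tick snaps the mesh to zero rotation in range (look-at nodes are unwired), easing back outside.
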(event Custom|StartDialogue
  (params (PlayerChar :type BP%20Player%20Character%20Object%20Reference))
  (bind _returnvalue (Transformation|GetActorLocation))
  (bind _returnvalue_2 (Game|GetPlayerController 0))
  (bind _playermark (Variables|Default|GetPlayerMark))
  (bind _returnvalue_3 (Transformation|GetWorldLocation _playermark))
  (bind _returnvalue_4 (Math|Rotator|FindLookatRotation _returnvalue_3 _returnvalue))
  (Default|SetInteractionPaused (Variables|/Game/Player_Programming/FirstPerson/Blueprints/BP_PlayerCharacter.BP_PlayerCharacter_C|GetBPC_Interaction PlayerChar) true)
  (Default|SetSwordDrawn PlayerChar false) ; sheathe sword during conversation
  (Transformation|SetActorLocationAndRotation PlayerChar _returnvalue_3 _returnvalue_4 false true)
  (Pawn|SetControlRotation _returnvalue_2 (Math|Rotator|MakeRotator 0.0 0.0 (.Yaw (Math|Rotator|BreakRotator _returnvalue_4))))
  (Game|Player|SetViewTargetwithBlend _returnvalue_2 self 0.0 "VTBlend_Linear" 0.0 false)
  (Input|DisableInput PlayerChar _returnvalue_2)
  (Variables|/Script/Engine.PlayerController|SetbShowMouseCursor _returnvalue_2 true)
  (Input|SetInputModeGameandUI _returnvalue_2 0 "DoNotLock" true false)
  (bind _returnvalue_5 (UserInterface|CreateWidget "/Game/Blueprints/Danny/DannyUI/DialogueUI/WBP_DIalogue.WBP_DIalogue_C" 0 self))
  (bind _output_get (Variables|Default|SetDialogueWidget _returnvalue_5))
  (UserInterface|Viewport|AddtoViewport _output_get 0)
  (bind _done (CallFunction|IsQuestDone?))
  (if (and _done (== (Variables|Default|GetStartRow) "QuestInProgress"))
    (Default|ShowNode _returnvalue_5 "QuestComplete")
    (else
      (Default|ShowNode _returnvalue_5 (Variables|Default|GetStartRow)))))

(event Custom|EndDialogue
  (params (PlayerChar :type BP%20Player%20Character%20Object%20Reference))
  (bind _returnvalue (Game|GetPlayerController 0))
  (Variables|Default|GetDialogueWidget ; checks if a dialogue still exists before trying to close one
    (:then
      (Default|SetInteractionPaused (Variables|/Game/Player_Programming/FirstPerson/Blueprints/BP_PlayerCharacter.BP_PlayerCharacter_C|GetBPC_Interaction PlayerChar) false)
      (Widget|RemovefromParent (Variables|Default|GetDialogueWidget))
      (Variables|Default|SetDialogueWidget 0)
      (Default|UpdateCameraMode (Variables|Default|GetPlayerBP))
      (Game|Player|SetViewTargetwithBlend _returnvalue (Game|GetPlayerCharacter 0) 0.0 "VTBlend_Linear" 0.0 false)
      (Input|EnableInput PlayerChar _returnvalue)
      (Variables|/Script/Engine.PlayerController|SetbShowMouseCursor _returnvalue false)
      (Input|SetInputModeGameOnly _returnvalue false))
    (:else)))

(event Custom|Dialogue%20Handler
  (params (Action :type Name))
  (bind _asplayer_game_instance (Utilities|Casting|CastToPlayerGameInstance (Game|GetGameInstance)))
  (switch name Action
    (:AcceptQuest
      (switch int (Variables|Default|GetQuestID)
        (:1
          (Variables|/Game/Player_Programming/FirstPerson/PlayerGameInstance.PlayerGameInstance_C|SetQuest%20Objective%201 _asplayer_game_instance true))
        (:2
          (Variables|/Game/Player_Programming/FirstPerson/PlayerGameInstance.PlayerGameInstance_C|SetQuest%20Objective%202%20%28Apple%29 _asplayer_game_instance true))
        (:3
          (Variables|/Game/Player_Programming/FirstPerson/PlayerGameInstance.PlayerGameInstance_C|SetQuest%20Objective%203%20%28Wall%29 _asplayer_game_instance true)))
      (Variables|Default|SetStartRow "QuestInProgress"))
    (:CompleteQuest
      (Variables|Default|SetStartRow "QuestDone"))))

(event EventBeginPlay
  (bind _asbp_player_character (Utilities|Casting|CastToBP_PlayerCharacter (Game|GetPlayerCharacter 0)))
  (Variables|Default|SetPlayerBP _asbp_player_character)
  (Variables|Default|SetOriginalRotation (Transformation|GetWorldRotation (Variables|Default|GetSkeletonMesh))))

(event EventTick
  (params (DeltaSeconds :type Float%20%28single-precision%29))
  (bind _skeletonmesh (Variables|Default|GetSkeletonMesh))
  ;[0.15 0.15 0.15 0.5] Look At Player in range
  (if (< (Transformation|GetDistanceTo (Game|GetPlayerCharacter 0)) (Variables|Default|GetDetectionRadius))
    (Transformation|SetWorldRotation _skeletonmesh "0, 0, 0" false false) ; if player in range, look at
    (else
      (Transformation|SetWorldRotation _skeletonmesh (Math|Interpolation|RInterpTo (Transformation|GetWorldRotation _skeletonmesh) (Variables|Default|GetOriginalRotation) DeltaSeconds 2.0) false false) ; if not, look at original direction
    )))

(event EventInteract
  (params (Interactor :type Actor%20Object%20Reference))
  (bind _playerbp (Variables|Default|GetPlayerBP))
  (CallFunction|StartDialogue _playerbp)
  (Development|PrintString "event interact fired")
  (Default|SetSwordDrawn _playerbp false))

(fn ConstructionScript)

(fn IsQuestDone?
  (bind _asplayer_game_instance (Utilities|Casting|CastToPlayerGameInstance (Game|GetGameInstance)))
  (switch int (Variables|Default|GetQuestID)
    (:1
      ;[0.15 0.15 0.15 0.5] NPC 1 Logic (Baskets)
      (if (>= (Variables|/Game/Player_Programming/FirstPerson/PlayerGameInstance.PlayerGameInstance_C|GetMats _asplayer_game_instance) (Variables|Default|GetMaterialsQuestGoal))
        (Variables|/Game/Player_Programming/FirstPerson/PlayerGameInstance.PlayerGameInstance_C|SetQuest%20Objective%201 _asplayer_game_instance false)
        (if (Variables|/Game/Player_Programming/FirstPerson/PlayerGameInstance.PlayerGameInstance_C|GetQuest%20One%20Completed _asplayer_game_instance)
          (Game|SpawnActorfromClass "/Game/Drops/QuestStuff/QuestRewardMaterials.QuestRewardMaterials_C" (Math|Transform|MakeTransform (Transformation|GetWorldLocation (Variables|Default|GetQuest%20Drop%20Location%20Reference))) "Undefined" "MultiplyWithRoot" 0 0)
          (else
            (Variables|/Game/Player_Programming/FirstPerson/PlayerGameInstance.PlayerGameInstance_C|SetQuest%20One%20Completed _asplayer_game_instance true)
            (Game|SpawnActorfromClass "/Game/Drops/NormalDrops/ExampleNormalDrop.ExampleNormalDrop_C" (Math|Transform|MakeTransform (Transformation|GetWorldLocation (Variables|Default|GetQuest%20Drop%20Location%20Reference))) "Undefined" "MultiplyWithRoot" 0 0)))
        (return (>= (Variables|/Game/Player_Programming/FirstPerson/PlayerGameInstance.PlayerGameInstance_C|GetMats _asplayer_game_instance) (Variables|Default|GetMaterialsQuestGoal)))))
    (:2
      ;[0.15 0.15 0.15 0.5] NPC 2 Logic (Apple)
      (if (Variables|/Game/Player_Programming/FirstPerson/PlayerGameInstance.PlayerGameInstance_C|GetApple _asplayer_game_instance)
        (Variables|/Game/Player_Programming/FirstPerson/PlayerGameInstance.PlayerGameInstance_C|SetQuest%20Objective%202%20%28Apple%29 _asplayer_game_instance false)
        (if (Variables|/Game/Player_Programming/FirstPerson/PlayerGameInstance.PlayerGameInstance_C|GetQuest%20Two%20Completed _asplayer_game_instance)
          (Game|SpawnActorfromClass "/Game/Drops/QuestStuff/QuestRewardMaterials.QuestRewardMaterials_C" (Math|Transform|MakeTransform (Transformation|GetWorldLocation (Variables|Default|GetQuest%20Drop%20Location%20Reference))) "Undefined" "MultiplyWithRoot" 0 0)
          (else
            (Variables|/Game/Player_Programming/FirstPerson/PlayerGameInstance.PlayerGameInstance_C|SetQuest%20Two%20Completed _asplayer_game_instance true)
            (Game|SpawnActorfromClass "/Game/Drops/NormalDrops/ExampleNormalDrop2.ExampleNormalDrop2_C" (Math|Transform|MakeTransform (Transformation|GetWorldLocation (Variables|Default|GetQuest%20Drop%20Location%20Reference))) "Undefined" "MultiplyWithRoot" 0 0)))
        (return (Variables|/Game/Player_Programming/FirstPerson/PlayerGameInstance.PlayerGameInstance_C|GetApple _asplayer_game_instance))))
    (:3
      ;[0.15 0.15 0.15 0.5] NPC 3 Logic (Debris)
      (if (Variables|/Game/Player_Programming/FirstPerson/PlayerGameInstance.PlayerGameInstance_C|GetQuest%20Objective%203%20%28Wall%29 _asplayer_game_instance)
        (Variables|/Game/Player_Programming/FirstPerson/PlayerGameInstance.PlayerGameInstance_C|SetQuest%20Objective%203%20%28Wall%29 _asplayer_game_instance false)
        (if (Variables|/Game/Player_Programming/FirstPerson/PlayerGameInstance.PlayerGameInstance_C|GetQuest%20Three%20Completed _asplayer_game_instance)
          (Game|SpawnActorfromClass "/Game/Drops/QuestStuff/QuestRewardMaterials.QuestRewardMaterials_C" (Math|Transform|MakeTransform (Transformation|GetWorldLocation (Variables|Default|GetQuest%20Drop%20Location%20Reference))) "Undefined" "MultiplyWithRoot" 0 0)
          (else
            (Variables|/Game/Player_Programming/FirstPerson/PlayerGameInstance.PlayerGameInstance_C|SetQuest%20Three%20Completed _asplayer_game_instance true)
            (Game|SpawnActorfromClass "/Game/Drops/NormalDrops/ExampleNormalDrop3.ExampleNormalDrop3_C" (Math|Transform|MakeTransform (Transformation|GetWorldLocation (Variables|Default|GetQuest%20Drop%20Location%20Reference))) "Undefined" "MultiplyWithRoot" 0 0)))
        (return (Variables|/Game/Player_Programming/FirstPerson/PlayerGameInstance.PlayerGameInstance_C|GetQuest%20Objective%203%20%28Wall%29 _asplayer_game_instance))))))

(fn CanInteract
  (params (Interactor :type Actor%20Object%20Reference))
  (return true))

(fn GetInteractionText
  (return "Talk"))