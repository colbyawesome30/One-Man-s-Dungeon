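; Player interaction component that finds nearby BPI_Interactable actors, shows a prompt and triggers interaction.
; A looping timer sphere-traces around the owner and keeps the hit actor as current if it allows interaction.
; Focus changes notify the interactable, update the widget and fire found/lost dispatchers.
; Interact rechecks eligibility before messaging the target and reporting success or failure, while SetInteractionPaused pauses the scan and hides the widget.
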(event Custom|SetInteractionPaused
  (params (Paused :type Boolean))
  (if Paused
    (Class|KismetSystemLibrary|PauseTimer 0 "TraceForInteractable")
    (Widget|SetVisibility (Variables|Default|GetInteractionWidgetRef) "Hidden")
    (else
      (Class|KismetSystemLibrary|UnPauseTimer 0 "TraceForInteractable")
      (Widget|SetVisibility (Variables|Default|GetInteractionWidgetRef) "Hidden"))))

(event EventBeginPlay
  (CallFunction|Interaction)
  (CallFunction|InteractionTrace))

(fn Interaction
  (bind _asbp_player_character (Utilities|Casting|CastToBP_PlayerCharacter (Game|GetPlayerCharacter 0)))
  (bind _output_get (Variables|Default|SetOwningCharacter _asbp_player_character))
  (bind _asplayer_controller (Utilities|Casting|CastToPlayerController (Pawn|GetController _output_get)))
  (bind _output_get_2 (Variables|Default|SetOwningController _asplayer_controller))
  (bind _returnvalue (UserInterface|CreateWidget (Variables|Default|GetInteractionWidgetClass) _output_get_2))
  (bind _output_get_3 (Variables|Default|SetInteractionWidgetRef _returnvalue))
  (UserInterface|Viewport|AddtoViewport _output_get_3 0)
  (Variables|/Script/UMG.Widget|SetVisibility _output_get_3 "Hidden"))

(fn SetCurrentInteractable
  (params (NewInteractable :type Actor%20Object%20Reference))
  (bind _interactionwidgetref (Variables|Default|GetInteractionWidgetRef))
  (if (not (== NewInteractable (Variables|Default|GetCurrentInteractable)))
    (Utilities|IsValid (Variables|Default|GetCurrentInteractable)
      (:Is%20Valid
        (Class|BPIInteractable|OnEndFocus(Message) (Variables|Default|GetCurrentInteractable) (Components|GetOwner)))
      (:Is%20Not%20Valid
        _))
    (bind _output_get (Variables|Default|SetCurrentInteractable NewInteractable))
    (Utilities|IsValid _output_get
      (:Is%20Valid
        (Class|BPIInteractable|OnBeginFocus(Message) (Variables|Default|GetCurrentInteractable) (Components|GetOwner))
        (bind _interactiontext (Class|BPIInteractable|GetInteractionText(Message) (Variables|Default|GetCurrentInteractable)))
        (Default|SetInteractionText _interactionwidgetref _interactiontext)
        (Variables|/Script/UMG.Widget|SetVisibility _interactionwidgetref "Visible")
        (Default|CallOnInteractableFound (Variables|Default|GetCurrentInteractable) _interactiontext))
      (:Is%20Not%20Valid
        (Variables|/Script/UMG.Widget|SetVisibility (Variables|Default|GetInteractionWidgetRef) "Hidden")
        (Default|CallOnInteractableLost)))))

(fn InteractionTrace
  (Utilities|Time|SetTimerbyFunctionName 0 "TraceForInteractable" 0.1 true))

(fn NewFunction)

(fn TraceforInteractable
  (bind _returnvalue (Components|GetOwner))
  (bind _returnvalue_2 (Transformation|GetActorLocation _returnvalue))
  (Utilities|IsValid _returnvalue
    (:Is%20Valid
      (bind (_outhit _returnvalue_3) (Collision|SphereTraceByChannel _returnvalue_2 _returnvalue_2 2e+02 (Variables|Default|GetTraceChannel) false (Utilities|Array|MakeArray _returnvalue) "None"))
      (if _returnvalue_3
        (if (Utilities|DoesObjectImplementInterface (.HitActor (Collision|BreakHitResult _outhit)) "/Game/Blueprints/Danny/DannyBlueprints/BPI_Interactable.BPI_Interactable_C")
          (bind _caninteract_ (Class|BPIInteractable|CanInteract(Message) (.HitActor (Collision|BreakHitResult _outhit)) (Components|GetOwner)))
          (if _caninteract_
            (CallFunction|SetCurrentInteractable (.HitActor (Collision|BreakHitResult _outhit)))
            (else
              (CallFunction|SetCurrentInteractable :!label _label)))
          (else
            (goto _label)))
        (else
          (goto _label))))))

(fn Interact
  (bind _returnvalue (Components|GetOwner))
  (bind _currentinteractable (Variables|Default|GetCurrentInteractable))
  (bind _currentinteractable_2 (Variables|Default|GetCurrentInteractable))
  (Utilities|IsValid _currentinteractable
    (:Is%20Valid
      (bind _caninteract_ (Class|BPIInteractable|CanInteract(Message) _currentinteractable _returnvalue))
      (if _caninteract_
        (Class|BPIInteractable|Interact(Message) _currentinteractable_2 _returnvalue)
        (Default|CallOnInteracted _currentinteractable_2)
        (else
          (Default|CallOnInteractFailed (Variables|Default|GetCurrentInteractable)))))
    (:Is%20Not%20Valid
      (Default|CallOnInteractFailed))))